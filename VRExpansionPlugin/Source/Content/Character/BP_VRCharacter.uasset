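; VR player character that drives animated Quest 3 controller models and supports hand-based climbing.
; BeginPlay resets HMD orientation and position, caches both controller anim instances and maps hand-interaction input; an input action repeats the reset.
; Trigger, grip, button and thumbstick actions write directly into those anim instances.
; UpdateClimbingMovement moves the body opposite the climbing hand's offset from its grip point through custom replicated VR movement.
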(event `self.ReceiveBeginPlay`
  (`HeadMountedDisplayFunctionLibrary.ResetOrientationAndPosition` 0.0)
  (bind _asabp_quest_3right_controller (cast `/VRExpansionPlugin/InitContent/Headset/Rigs/ABP_Quest3RightController` (`SkeletalMeshComponent.GetAnimInstance` (`self.HandMeshRight`))))
  (set `self.RightControllerAnimInstance` _asabp_quest_3right_controller)
  (bind _asabp_quest_3left_controller (cast `/VRExpansionPlugin/InitContent/Headset/Rigs/ABP_Quest3LeftController` (`SkeletalMeshComponent.GetAnimInstance` (`self.HandMeshLeft`))))
  (set `self.LeftControllerAnimInstance` _asabp_quest_3left_controller)
  (`self.MapInput` "/VRExpansionPlugin/Inputs/IMC_HandInteractions.IMC_HandInteractions"))

(event `EnhancedInput|/VRExpansionPlugin/Inputs/CharacterInputs/IA_ResetOrientation`
  (params (ActionValue :type Boolean) (ElapsedSeconds :type "Float (double-precision)") (TriggeredSeconds :type "Float (double-precision)") (InputAction :type "InputAction Object Reference" :default "/VRExpansionPlugin/Inputs/CharacterInputs/IA_ResetOrientation.IA_ResetOrientation"))
  (:`Triggered`
    (`HeadMountedDisplayFunctionLibrary.ResetOrientationAndPosition` 0.0)))

(event `self.UpdateClimbingMovement`
  (params (DeltaTime :type "Float (single-precision)"))
  ;[0.4973 1 0.4305] Climbing
  (if (`self.bIsClimbing`)
    (`self.ClimbingHand`
      (:`then`
        (`self.ClimbingGrip`
          (:`then`
            (`VRBaseCharacterMovementComponent.AddCustomReplicatedMovement` (`self.VRMovementReference`) (`KismetMathLibrary.NegateVector` (- (`SceneComponent.K2_GetComponentLocation` (`self.ClimbingHand`)) (`KismetMathLibrary.TransformLocation` (`SceneComponent.K2_GetComponentToWorld` (`self.ClimbingGrip`)) (`self.ClimbGripLocation`))))))
          (:`else`)))
      (:`else`))))

(event `EnhancedInput|/VRExpansionPlugin/Inputs/HandInteractionsInput/ButtonInputs/IA_LeftHandTrigger`
  (params (ActionValue :type "Float (double-precision)") (ElapsedSeconds :type "Float (double-precision)") (TriggeredSeconds :type "Float (double-precision)") (InputAction :type "InputAction Object Reference" :default "/VRExpansionPlugin/Inputs/HandInteractionsInput/ButtonInputs/IA_LeftHandTrigger.IA_LeftHandTrigger"))
  (bind _leftcontrolleraniminstance (`self.LeftControllerAnimInstance`))
  ;[1 1 1] Button Hand Interactions
  (:`Triggered`
    (set `/VRExpansionPlugin/InitContent/Headset/Rigs/ABP_Quest3LeftController.TriggerAlpha` ActionValue _leftcontrolleraniminstance))
  (:`Completed`
    (set `/VRExpansionPlugin/InitContent/Headset/Rigs/ABP_Quest3LeftController.TriggerAlpha` 0.0 _leftcontrolleraniminstance)))

(event `EnhancedInput|/VRExpansionPlugin/Inputs/HandInteractionsInput/ButtonInputs/IA_RightHandTrigger`
  (params (ActionValue :type "Float (double-precision)") (ElapsedSeconds :type "Float (double-precision)") (TriggeredSeconds :type "Float (double-precision)") (InputAction :type "InputAction Object Reference" :default "/VRExpansionPlugin/Inputs/HandInteractionsInput/ButtonInputs/IA_RightHandTrigger.IA_RightHandTrigger"))
  (bind _rightcontrolleraniminstance (`self.RightControllerAnimInstance`))
  ;[1 1 1] Button Hand Interactions
  (:`Triggered`
    (set `/VRExpansionPlugin/InitContent/Headset/Rigs/ABP_Quest3RightController.TriggerAlpha` ActionValue _rightcontrolleraniminstance))
  (:`Completed`
    (set `/VRExpansionPlugin/InitContent/Headset/Rigs/ABP_Quest3RightController.TriggerAlpha` 0.0 _rightcontrolleraniminstance)))

(event `EnhancedInput|/VRExpansionPlugin/Inputs/HandInteractionsInput/ButtonInputs/IA_LeftHandGrip`
  (params (ActionValue :type "Float (double-precision)") (ElapsedSeconds :type "Float (double-precision)") (TriggeredSeconds :type "Float (double-precision)") (InputAction :type "InputAction Object Reference" :default "/VRExpansionPlugin/Inputs/HandInteractionsInput/ButtonInputs/IA_LeftHandGrip.IA_LeftHandGrip"))
  (bind _leftcontrolleraniminstance (`self.LeftControllerAnimInstance`))
  ;[1 1 1] Button Hand Interactions
  (:`Triggered`
    (set `/VRExpansionPlugin/InitContent/Headset/Rigs/ABP_Quest3LeftController.GripAlpha` ActionValue _leftcontrolleraniminstance))
  (:`Completed`
    (set `/VRExpansionPlugin/InitContent/Headset/Rigs/ABP_Quest3LeftController.GripAlpha` 0.0 _leftcontrolleraniminstance)))

(event `EnhancedInput|/VRExpansionPlugin/Inputs/HandInteractionsInput/ButtonInputs/IA_RightHandGrip`
  (params (ActionValue :type "Float (double-precision)") (ElapsedSeconds :type "Float (double-precision)") (TriggeredSeconds :type "Float (double-precision)") (InputAction :type "InputAction Object Reference" :default "/VRExpansionPlugin/Inputs/HandInteractionsInput/ButtonInputs/IA_RightHandGrip.IA_RightHandGrip"))
  (bind _rightcontrolleraniminstance (`self.RightControllerAnimInstance`))
  ;[1 1 1] Button Hand Interactions
  (:`Triggered`
    (set `/VRExpansionPlugin/InitContent/Headset/Rigs/ABP_Quest3RightController.GripAlpha` ActionValue _rightcontrolleraniminstance))
  (:`Completed`
    (set `/VRExpansionPlugin/InitContent/Headset/Rigs/ABP_Quest3RightController.GripAlpha` 0.0 _rightcontrolleraniminstance)))

(event `EnhancedInput|/VRExpansionPlugin/Inputs/HandInteractionsInput/ButtonInputs/IA_LeftHandPrimaryButton`
  (params (ActionValue :type Boolean) (ElapsedSeconds :type "Float (double-precision)") (TriggeredSeconds :type "Float (double-precision)") (InputAction :type "InputAction Object Reference" :default "/VRExpansionPlugin/Inputs/HandInteractionsInput/ButtonInputs/IA_LeftHandPrimaryButton.IA_LeftHandPrimaryButton"))
  (bind _leftcontrolleraniminstance (`self.LeftControllerAnimInstance`))
  ;[1 1 1] Button Hand Interactions
  (:`Triggered`
    (set `/VRExpansionPlugin/InitContent/Headset/Rigs/ABP_Quest3LeftController.PrimaryButton` true _leftcontrolleraniminstance))
  (:`Completed`
    (set `/VRExpansionPlugin/InitContent/Headset/Rigs/ABP_Quest3LeftController.PrimaryButton` false _leftcontrolleraniminstance)))

(event `EnhancedInput|/VRExpansionPlugin/Inputs/HandInteractionsInput/ButtonInputs/IA_RightHandPrimaryButton`
  (params (ActionValue :type Boolean) (ElapsedSeconds :type "Float (double-precision)") (TriggeredSeconds :type "Float (double-precision)") (InputAction :type "InputAction Object Reference" :default "/VRExpansionPlugin/Inputs/HandInteractionsInput/ButtonInputs/IA_RightHandPrimaryButton.IA_RightHandPrimaryButton"))
  (bind _rightcontrolleraniminstance (`self.RightControllerAnimInstance`))
  ;[1 1 1] Button Hand Interactions
  (:`Triggered`
    (set `/VRExpansionPlugin/InitContent/Headset/Rigs/ABP_Quest3RightController.PrimaryButton` true _rightcontrolleraniminstance))
  (:`Completed`
    (set `/VRExpansionPlugin/InitContent/Headset/Rigs/ABP_Quest3RightController.PrimaryButton` false _rightcontrolleraniminstance)))

(event `EnhancedInput|/VRExpansionPlugin/Inputs/HandInteractionsInput/ButtonInputs/IA_LeftHandSecondaryButton`
  (params (ActionValue :type Boolean) (ElapsedSeconds :type "Float (double-precision)") (TriggeredSeconds :type "Float (double-precision)") (InputAction :type "InputAction Object Reference" :default "/VRExpansionPlugin/Inputs/HandInteractionsInput/ButtonInputs/IA_LeftHandSecondaryButton.IA_LeftHandSecondaryButton"))
  (bind _leftcontrolleraniminstance (`self.LeftControllerAnimInstance`))
  ;[1 1 1] Button Hand Interactions
  (:`Triggered`
    (set `/VRExpansionPlugin/InitContent/Headset/Rigs/ABP_Quest3LeftController.SecondaryButton` true _leftcontrolleraniminstance))
  (:`Completed`
    (set `/VRExpansionPlugin/InitContent/Headset/Rigs/ABP_Quest3LeftController.SecondaryButton` true _leftcontrolleraniminstance)))

(event `EnhancedInput|/VRExpansionPlugin/Inputs/HandInteractionsInput/ButtonInputs/IA_RightHandSecondaryButton`
  (params (ActionValue :type Boolean) (ElapsedSeconds :type "Float (double-precision)") (TriggeredSeconds :type "Float (double-precision)") (InputAction :type "InputAction Object Reference" :default "/VRExpansionPlugin/Inputs/HandInteractionsInput/ButtonInputs/IA_RightHandSecondaryButton.IA_RightHandSecondaryButton"))
  (bind _rightcontrolleraniminstance (`self.RightControllerAnimInstance`))
  ;[1 1 1] Button Hand Interactions
  (:`Triggered`
    (set `/VRExpansionPlugin/InitContent/Headset/Rigs/ABP_Quest3RightController.SecondaryButton` true _rightcontrolleraniminstance))
  (:`Completed`
    (set `/VRExpansionPlugin/InitContent/Headset/Rigs/ABP_Quest3RightController.SecondaryButton` false _rightcontrolleraniminstance)))

(event `EnhancedInput|/VRExpansionPlugin/Inputs/HandInteractionsInput/ButtonInputs/IA_LeftHandThumbstick`
  (params (ActionValue :type "Vector2D Structure") (ElapsedSeconds :type "Float (double-precision)") (TriggeredSeconds :type "Float (double-precision)") (InputAction :type "InputAction Object Reference" :default "/VRExpansionPlugin/Inputs/HandInteractionsInput/ButtonInputs/IA_LeftHandThumbstick.IA_LeftHandThumbstick"))
  (bind _leftcontrolleraniminstance (`self.LeftControllerAnimInstance`))
  ;[1 1 1] Button Hand Interactions
  (:`Triggered`
    (set `/VRExpansionPlugin/InitContent/Headset/Rigs/ABP_Quest3LeftController.ThumbStick` ActionValue _leftcontrolleraniminstance))
  (:`Completed`
    (set `/VRExpansionPlugin/InitContent/Headset/Rigs/ABP_Quest3LeftController.ThumbStick` (0.0 0.0) _leftcontrolleraniminstance)))

(event `EnhancedInput|/VRExpansionPlugin/Inputs/HandInteractionsInput/ButtonInputs/IA_RightHandThumbstick`
  (params (ActionValue :type "Vector2D Structure") (ElapsedSeconds :type "Float (double-precision)") (TriggeredSeconds :type "Float (double-precision)") (InputAction :type "InputAction Object Reference" :default "/VRExpansionPlugin/Inputs/HandInteractionsInput/ButtonInputs/IA_RightHandThumbstick.IA_RightHandThumbstick"))
  (bind _rightcontrolleraniminstance (`self.RightControllerAnimInstance`))
  ;[1 1 1] Button Hand Interactions
  (:`Triggered`
    (set `/VRExpansionPlugin/InitContent/Headset/Rigs/ABP_Quest3RightController.ThumbStick` ActionValue _rightcontrolleraniminstance))
  (:`Completed`
    (set `/VRExpansionPlugin/InitContent/Headset/Rigs/ABP_Quest3RightController.ThumbStick` (0.0 0.0) _rightcontrolleraniminstance)))

(event `EnhancedInput|/VRExpansionPlugin/Inputs/HandInteractionsInput/ButtonInputs/IA_LeftHandMenuButton`
  (params (ActionValue :type Boolean) (ElapsedSeconds :type "Float (double-precision)") (TriggeredSeconds :type "Float (double-precision)") (InputAction :type "InputAction Object Reference" :default "/VRExpansionPlugin/Inputs/HandInteractionsInput/ButtonInputs/IA_LeftHandMenuButton.IA_LeftHandMenuButton"))
  (bind _leftcontrolleraniminstance (`self.LeftControllerAnimInstance`))
  ;[1 1 1] Button Hand Interactions
  (:`Triggered`
    (set `/VRExpansionPlugin/InitContent/Headset/Rigs/ABP_Quest3LeftController.SpecialButton` true _leftcontrolleraniminstance))
  (:`Completed`
    (set `/VRExpansionPlugin/InitContent/Headset/Rigs/ABP_Quest3LeftController.SpecialButton` true _leftcontrolleraniminstance)))

(fn `UserConstructionScript`)