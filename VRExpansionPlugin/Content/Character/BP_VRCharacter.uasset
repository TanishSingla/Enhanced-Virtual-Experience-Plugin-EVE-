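; VR player character that drives Quest 3 controller animations and optionally spawns physically grasping hands.
; On BeginPlay it spawns GraspingHandManny actors on both motion controllers under OpenXR, hiding the default hand meshes, then resets orientation.
; It caches both controller anim instances and maps hand-interaction input.
; Enhanced Input events write trigger, grip, button and thumbstick states into those instances, though the left thumbstick is always written as zero.
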(event `self.ReceiveBeginPlay`
  (bind _returnvalue (`self.CheckXRApi`))
  (if (`KismetStringLibrary.EqualEqual_StrStr` _returnvalue "OpenXR")
    (`self.CheckSpawnGraspingHands`))
  (`HeadMountedDisplayFunctionLibrary.ResetOrientationAndPosition` 0.0)
  (`self.EnableControllerAnimations`))

(event `EnhancedInput|/VRExpansionPlugin/Inputs/HandInteractionsInput/ButtonInputs/IA_LeftHandTrigger`
  (params (ActionValue :type "Float (double-precision)") (ElapsedSeconds :type "Float (double-precision)") (TriggeredSeconds :type "Float (double-precision)") (InputAction :type "InputAction Object Reference" :default "/VRExpansionPlugin/Inputs/HandInteractionsInput/ButtonInputs/IA_LeftHandTrigger.IA_LeftHandTrigger"))
  (bind _leftcontrolleraniminstance (`self.LeftControllerAnimInstance`))
  ;[1 1 1] Button Hand Interactions
  (:`Triggered`
    (set `/VRExpansionPlugin/InitContent/Headset/Rigs/ABP_Quest3LeftController.TriggerAlpha` ActionValue _leftcontrolleraniminstance))
  (:`Completed`
    (set `/VRExpansionPlugin/InitContent/Headset/Rigs/ABP_Quest3LeftController.TriggerAlpha` 0.0 _leftcontrolleraniminstance)))

(event `EnhancedInput|/VRExpansionPlugin/Inputs/HandInteractionsInput/ButtonInputs/IA_RightHandTrigger`
  (params (ActionValue :type "Float (double-precision)") (ElapsedSeconds :type "Float (double-precision)") (TriggeredSeconds :type "Float (double-precision)") (InputAction :type "InputAction Object Reference" :default "/VRExpansionPlugin/Inputs/HandInteractionsInput/ButtonInputs/IA_RightHandTrigger.IA_RightHandTrigger"))
  (bind _rightcontrolleraniminstance (`self.RightControllerAnimInstance`))
  ;[1 1 1] Button Hand Interactions
  (:`Triggered`
    (set `/VRExpansionPlugin/InitContent/Headset/Rigs/ABP_Quest3RightController.TriggerAlpha` ActionValue _rightcontrolleraniminstance))
  (:`Completed`
    (set `/VRExpansionPlugin/InitContent/Headset/Rigs/ABP_Quest3RightController.TriggerAlpha` 0.0 _rightcontrolleraniminstance)))

(event `EnhancedInput|/VRExpansionPlugin/Inputs/HandInteractionsInput/ButtonInputs/IA_LeftHandGrip`
  (params (ActionValue :type "Float (double-precision)") (ElapsedSeconds :type "Float (double-precision)") (TriggeredSeconds :type "Float (double-precision)") (InputAction :type "InputAction Object Reference" :default "/VRExpansionPlugin/Inputs/HandInteractionsInput/ButtonInputs/IA_LeftHandGrip.IA_LeftHandGrip"))
  (bind _leftcontrolleraniminstance (`self.LeftControllerAnimInstance`))
  ;[1 1 1] Button Hand Interactions
  (:`Triggered`
    (set `/VRExpansionPlugin/InitContent/Headset/Rigs/ABP_Quest3LeftController.GripAlpha` ActionValue _leftcontrolleraniminstance))
  (:`Completed`
    (set `/VRExpansionPlugin/InitContent/Headset/Rigs/ABP_Quest3LeftController.GripAlpha` 0.0 _leftcontrolleraniminstance)))

(event `EnhancedInput|/VRExpansionPlugin/Inputs/HandInteractionsInput/ButtonInputs/IA_RightHandGrip`
  (params (ActionValue :type "Float (double-precision)") (ElapsedSeconds :type "Float (double-precision)") (TriggeredSeconds :type "Float (double-precision)") (InputAction :type "InputAction Object Reference" :default "/VRExpansionPlugin/Inputs/HandInteractionsInput/ButtonInputs/IA_RightHandGrip.IA_RightHandGrip"))
  (bind _rightcontrolleraniminstance (`self.RightControllerAnimInstance`))
  ;[1 1 1] Button Hand Interactions
  (:`Triggered`
    (set `/VRExpansionPlugin/InitContent/Headset/Rigs/ABP_Quest3RightController.GripAlpha` ActionValue _rightcontrolleraniminstance))
  (:`Completed`
    (set `/VRExpansionPlugin/InitContent/Headset/Rigs/ABP_Quest3RightController.GripAlpha` 0.0 _rightcontrolleraniminstance)))

(event `EnhancedInput|/VRExpansionPlugin/Inputs/HandInteractionsInput/ButtonInputs/IA_LeftHandPrimaryButton`
  (params (ActionValue :type Boolean) (ElapsedSeconds :type "Float (double-precision)") (TriggeredSeconds :type "Float (double-precision)") (InputAction :type "InputAction Object Reference" :default "/VRExpansionPlugin/Inputs/HandInteractionsInput/ButtonInputs/IA_LeftHandPrimaryButton.IA_LeftHandPrimaryButton"))
  (bind _leftcontrolleraniminstance (`self.LeftControllerAnimInstance`))
  ;[1 1 1] Button Hand Interactions
  (:`Triggered`
    (set `/VRExpansionPlugin/InitContent/Headset/Rigs/ABP_Quest3LeftController.PrimaryButton` ActionValue _leftcontrolleraniminstance))
  (:`Completed`
    (set `/VRExpansionPlugin/InitContent/Headset/Rigs/ABP_Quest3LeftController.PrimaryButton` ActionValue _leftcontrolleraniminstance)))

(event `EnhancedInput|/VRExpansionPlugin/Inputs/HandInteractionsInput/ButtonInputs/IA_RightHandPrimaryButton`
  (params (ActionValue :type Boolean) (ElapsedSeconds :type "Float (double-precision)") (TriggeredSeconds :type "Float (double-precision)") (InputAction :type "InputAction Object Reference" :default "/VRExpansionPlugin/Inputs/HandInteractionsInput/ButtonInputs/IA_RightHandPrimaryButton.IA_RightHandPrimaryButton"))
  (bind _rightcontrolleraniminstance (`self.RightControllerAnimInstance`))
  ;[1 1 1] Button Hand Interactions
  (:`Triggered`
    (set `/VRExpansionPlugin/InitContent/Headset/Rigs/ABP_Quest3RightController.PrimaryButton` ActionValue _rightcontrolleraniminstance))
  (:`Completed`
    (set `/VRExpansionPlugin/InitContent/Headset/Rigs/ABP_Quest3RightController.PrimaryButton` ActionValue _rightcontrolleraniminstance)))

(event `EnhancedInput|/VRExpansionPlugin/Inputs/HandInteractionsInput/ButtonInputs/IA_LeftHandSecondaryButton`
  (params (ActionValue :type Boolean) (ElapsedSeconds :type "Float (double-precision)") (TriggeredSeconds :type "Float (double-precision)") (InputAction :type "InputAction Object Reference" :default "/VRExpansionPlugin/Inputs/HandInteractionsInput/ButtonInputs/IA_LeftHandSecondaryButton.IA_LeftHandSecondaryButton"))
  (bind _leftcontrolleraniminstance (`self.LeftControllerAnimInstance`))
  ;[1 1 1] Button Hand Interactions
  (:`Triggered`
    (set `/VRExpansionPlugin/InitContent/Headset/Rigs/ABP_Quest3LeftController.SecondaryButton` ActionValue _leftcontrolleraniminstance))
  (:`Completed`
    (set `/VRExpansionPlugin/InitContent/Headset/Rigs/ABP_Quest3LeftController.SecondaryButton` ActionValue _leftcontrolleraniminstance)))

(event `EnhancedInput|/VRExpansionPlugin/Inputs/HandInteractionsInput/ButtonInputs/IA_RightHandSecondaryButton`
  (params (ActionValue :type Boolean) (ElapsedSeconds :type "Float (double-precision)") (TriggeredSeconds :type "Float (double-precision)") (InputAction :type "InputAction Object Reference" :default "/VRExpansionPlugin/Inputs/HandInteractionsInput/ButtonInputs/IA_RightHandSecondaryButton.IA_RightHandSecondaryButton"))
  (bind _rightcontrolleraniminstance (`self.RightControllerAnimInstance`))
  ;[1 1 1] Button Hand Interactions
  (:`Triggered`
    (set `/VRExpansionPlugin/InitContent/Headset/Rigs/ABP_Quest3RightController.SecondaryButton` ActionValue _rightcontrolleraniminstance))
  (:`Completed`
    (set `/VRExpansionPlugin/InitContent/Headset/Rigs/ABP_Quest3RightController.SecondaryButton` ActionValue _rightcontrolleraniminstance)))

(event `EnhancedInput|/VRExpansionPlugin/Inputs/HandInteractionsInput/ButtonInputs/IA_LeftHandThumbstick`
  (params (ActionValue :type "Vector2D Structure") (ElapsedSeconds :type "Float (double-precision)") (TriggeredSeconds :type "Float (double-precision)") (InputAction :type "InputAction Object Reference" :default "/VRExpansionPlugin/Inputs/HandInteractionsInput/ButtonInputs/IA_LeftHandThumbstick.IA_LeftHandThumbstick"))
  (bind _leftcontrolleraniminstance (`self.LeftControllerAnimInstance`))
  ;[1 1 1] Button Hand Interactions
  (:`Triggered`
    (set `/VRExpansionPlugin/InitContent/Headset/Rigs/ABP_Quest3LeftController.ThumbStick` (0.0 0.0) _leftcontrolleraniminstance))
  (:`Completed`
    (set `/VRExpansionPlugin/InitContent/Headset/Rigs/ABP_Quest3LeftController.ThumbStick` (0.0 0.0) _leftcontrolleraniminstance)))

(event `EnhancedInput|/VRExpansionPlugin/Inputs/HandInteractionsInput/ButtonInputs/IA_RightHandThumbstick`
  (params (ActionValue :type "Vector2D Structure") (ElapsedSeconds :type "Float (double-precision)") (TriggeredSeconds :type "Float (double-precision)") (InputAction :type "InputAction Object Reference" :default "/VRExpansionPlugin/Inputs/HandInteractionsInput/ButtonInputs/IA_RightHandThumbstick.IA_RightHandThumbstick"))
  (bind _rightcontrolleraniminstance (`self.RightControllerAnimInstance`))
  ;[1 1 1] Button Hand Interactions
  (:`Triggered`
    (set `/VRExpansionPlugin/InitContent/Headset/Rigs/ABP_Quest3RightController.ThumbStick` ActionValue _rightcontrolleraniminstance))
  (:`Completed`
    (set `/VRExpansionPlugin/InitContent/Headset/Rigs/ABP_Quest3RightController.ThumbStick` (0.0 0.0) _rightcontrolleraniminstance)))

(event `EnhancedInput|/VRExpansionPlugin/Inputs/HandInteractionsInput/ButtonInputs/IA_LeftHandMenuButton`
  (params (ActionValue :type Boolean) (ElapsedSeconds :type "Float (double-precision)") (TriggeredSeconds :type "Float (double-precision)") (InputAction :type "InputAction Object Reference" :default "/VRExpansionPlugin/Inputs/HandInteractionsInput/ButtonInputs/IA_LeftHandMenuButton.IA_LeftHandMenuButton"))
  (bind _leftcontrolleraniminstance (`self.LeftControllerAnimInstance`))
  ;[1 1 1] Button Hand Interactions
  (:`Triggered`
    (set `/VRExpansionPlugin/InitContent/Headset/Rigs/ABP_Quest3LeftController.SpecialButton` true _leftcontrolleraniminstance))
  (:`Completed`
    (set `/VRExpansionPlugin/InitContent/Headset/Rigs/ABP_Quest3LeftController.SpecialButton` false _leftcontrolleraniminstance)))

(fn `CheckSpawnGraspingHands`
  (locals (SpawnGraspingHands :type Boolean :default true) (GraspingHandsUseFingerCurls :type Boolean) (UsePhysicalGraspingHands :type Boolean :default false))
  (bind _leftmotioncontroller (`self.LeftMotionController`))
  (bind _rightmotioncontroller (`self.RightMotionController`))
  (if (`local.SpawnGraspingHands`)
    (`|ExecutionSequence`
      (:`then_0`
        ;[1 1 1] Clear the grasping hands so we can re-init them
        (`/Engine/EditorBlueprintResources/StandardMacros.IsValid` null :!label _label
          (:`Is Valid`
            (`self.K2_DestroyActor` null)
            (`/Engine/EditorBlueprintResources/ActorMacros.Switch Has Authority`
              (:`Remote`
                (`SceneComponent.SetHiddenInGame` (`self.HandMeshRight`) false false))))
          (:`Is Not Valid`
            _))
        (`/Engine/EditorBlueprintResources/StandardMacros.IsValid` null
          (:`Is Valid`
            (`self.K2_DestroyActor` null)
            (`/Engine/EditorBlueprintResources/ActorMacros.Switch Has Authority`
              (:`Remote`
                (`SceneComponent.SetHiddenInGame` (`self.HandMeshLeft`) false false))))
          (:`Is Not Valid`
            _))
        (`self.SetGripComponents` (`self.LeftGrabSphere`) (`self.RightGrabSphere`)))
      (:`then_1`
        (bind _returnvalue (`|SpawnActorFromClass` "/VRExpansionPlugin/VRHands/GraspingHandManny.GraspingHandManny_C" (`SceneComponent.K2_GetComponentToWorld` (`self.HandMeshRight`)) "Undefined" "MultiplyWithRoot" self _rightmotioncontroller (select `bool` (`local.UsePhysicalGraspingHands`) :`true` (`self.RightGrabSphere`)) (`self.LeftMotionController`) (`local.GraspingHandsUseFingerCurls`) self))
        (set `self.GraspingHandRight` _returnvalue)
        (`self.K2_AttachToComponent` _returnvalue _rightmotioncontroller "None" "KeepWorld" "KeepWorld" "KeepWorld" false)
        (`SceneComponent.SetHiddenInGame` (`self.RightGrabSphere`) true false)
        (`SceneComponent.SetHiddenInGame` (`self.HandMeshRight`) true false)
        (bind _returnvalue_2 (`|SpawnActorFromClass` "/VRExpansionPlugin/VRHands/GraspingHandManny.GraspingHandManny_C" (`SceneComponent.K2_GetComponentToWorld` (`self.HandMeshLeft`)) "Undefined" "MultiplyWithRoot" self _leftmotioncontroller (select `bool` (`local.UsePhysicalGraspingHands`) :`true` (`self.LeftGrabSphere`)) (`self.RightMotionController`) (`local.GraspingHandsUseFingerCurls`) self))
        (set `self.GraspingHandLeft` _returnvalue_2)
        (`self.K2_AttachToComponent` _returnvalue_2 _leftmotioncontroller "None" "KeepWorld" "KeepWorld" "KeepWorld" false)
        (`SceneComponent.SetHiddenInGame` (`self.HandMeshLeft`) true false)
        (`SceneComponent.SetHiddenInGame` (`self.LeftGrabSphere`) true false)))
    (else
      (goto _label))))

(fn `EnableControllerAnimations`
  (bind _asabp_quest_3right_controller (cast `/VRExpansionPlugin/InitContent/Headset/Rigs/ABP_Quest3RightController` (`SkeletalMeshComponent.GetAnimInstance` (`self.HandMeshRight`))))
  (set `self.RightControllerAnimInstance` _asabp_quest_3right_controller)
  (bind _asabp_quest_3left_controller (cast `/VRExpansionPlugin/InitContent/Headset/Rigs/ABP_Quest3LeftController` (`SkeletalMeshComponent.GetAnimInstance` (`self.HandMeshLeft`))))
  (set `self.LeftControllerAnimInstance` _asabp_quest_3left_controller)
  (`self.MapInput` "/VRExpansionPlugin/Inputs/IMC_HandInteractions.IMC_HandInteractions" 1))

(fn `UserConstructionScript`)