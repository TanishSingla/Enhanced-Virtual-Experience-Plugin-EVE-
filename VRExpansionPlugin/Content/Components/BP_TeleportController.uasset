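; BP_TeleportController handles the trigger input for physics-tossing objects highlighted by a laser in a motion-controller setup.
; On right-hand trigger press, it checks that the laser is active, no throw is in progress and the widget interaction component is off interactable or focusable widgets.
; It then passes any valid highlighted object and the owning motion controller to PhysicsTossManager's ServersideToss.
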(event `EnhancedInput|/VRExpansionPlugin/Inputs/HandInteractionsInput/ButtonInputs/IA_RightHandTrigger`
  (params (ActionValue :type "Float (double-precision)") (ElapsedSeconds :type "Float (double-precision)") (TriggeredSeconds :type "Float (double-precision)") (InputAction :type "InputAction Object Reference" :default "/VRExpansionPlugin/Inputs/HandInteractionsInput/ButtonInputs/IA_RightHandTrigger.IA_RightHandTrigger"))
  (bind _laserhighlightingobject (`self.LaserHighlightingObject`))
  (bind _wic (`self.Wic`))
  ;[0.5016 0.9301 1] Physics Toss
  (:`Started`
    (if (and (`self.bIsLaserBeamActive`) (not (`/VRExpansionPlugin/Components/PhysicsTossManager.IsThrowing` (`self.PhysicsTossManager`))) (`KismetMathLibrary.BooleanNOR` (`WidgetInteractionComponent.IsOverInteractableWidget` _wic) (`WidgetInteractionComponent.IsOverFocusableWidget` _wic)))
      (`/Engine/EditorBlueprintResources/StandardMacros.IsValid` _laserhighlightingobject
        (:`Is Valid`
          (`/VRExpansionPlugin/Components/PhysicsTossManager.ServersideToss` (`self.PhysicsTossManager`) _laserhighlightingobject (`self.OwningMotionController`)))))))

(fn `UserConstructionScript`)