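; BP_TeleportController is a per-hand VR controller helper handling laser physics tosses and hand-based widget interaction.
; On grab trigger, the active laser's highlighted object goes to PhysicsTossManager for a server-side toss, unless over interactable or focusable widgets.
; After a short BeginPlay delay, it binds to its side's GraspingHand events.
; These feed hit results into the widget interaction component to press and release widgets, with haptic feedback.
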(event `self.GrabTrigger`
  (bind _laserhighlightingobject (`self.LaserHighlightingObject`))
  (bind _wic (`self.Wic`))
  ;[0.5016 0.9301 1] Physics Toss
  (if (and (`self.bIsLaserBeamActive`) (not (`/EnhancedVirtualExperience/Components/PhysicsTossManager.IsThrowing` (`self.PhysicsTossManager`))) (`KismetMathLibrary.BooleanNOR` (`WidgetInteractionComponent.IsOverInteractableWidget` _wic) (`WidgetInteractionComponent.IsOverFocusableWidget` _wic)))
    (`/Engine/EditorBlueprintResources/StandardMacros.IsValid` _laserhighlightingobject
      (:`Is Valid`
        (`/EnhancedVirtualExperience/Components/PhysicsTossManager.ServersideToss` (`self.PhysicsTossManager`) _laserhighlightingobject (`self.OwningMotionController`))))))

(event `self.ReceiveBeginPlay`
  ;[0.4297 1 0.9701] WidgetInteractionWithHand Logic
  (`KismetSystemLibrary.Delay` 0.1)
  (bind _asbp_vrcharacter (cast `/EnhancedVirtualExperience/Character/BP_VRCharacter` (`GameplayStatics.GetPlayerPawn` 0)))
  (switch `EControllerHand` (`GripMotionControllerComponent.GetHandType` (`self.OwningMotionController`))
    (:`Left`
      (bind _graspinghandleft (`/EnhancedVirtualExperience/Character/BP_VRCharacter.GraspingHandLeft` _asbp_vrcharacter)
        (:`then`
          (add `/EnhancedVirtualExperience/VRHands/GraspingHandManny.OnStartInteraction` _graspinghandleft (delegate `OnLeftStartInteraction`))
          (add `/EnhancedVirtualExperience/VRHands/GraspingHandManny.OnEndInteraction` _graspinghandleft (delegate `OnLeftEndInteraction`)))
        (:`else`)))
    (:`Right`
      (bind _graspinghandright (`/EnhancedVirtualExperience/Character/BP_VRCharacter.GraspingHandRight` _asbp_vrcharacter)
        (:`then`
          (add `/EnhancedVirtualExperience/VRHands/GraspingHandManny.OnStartInteraction` _graspinghandright (delegate `OnRightStartInteraction`))
          (add `/EnhancedVirtualExperience/VRHands/GraspingHandManny.OnEndInteraction` _graspinghandright (delegate `OnRightEndInteraction`)))
        (:`else`)))))

(event `OnLeftStartInteraction`
  (params (HitResult :type "HitResult Structure"))
  ;[0.4297 1 0.9701] WidgetInteractionWithHand Logic
  (`self.OnWidgetHandStartInteraction` HitResult))

(event `OnLeftEndInteraction`
  ;[0.4297 1 0.9701] WidgetInteractionWithHand Logic
  (`self.OnWidgetHandEndInteraction`))

(event `OnRightStartInteraction`
  (params (HitResult :type "HitResult Structure"))
  ;[0.4297 1 0.9701] WidgetInteractionWithHand Logic
  (`self.OnWidgetHandStartInteraction` HitResult))

(event `OnRightEndInteraction`
  ;[0.4297 1 0.9701] WidgetInteractionWithHand Logic
  (`self.OnWidgetHandEndInteraction`))

(fn `OnWidgetHandEndInteraction`
  (`self.IfOverWidgetUse` false true)
  (`self.DisableWidgetActivation`))

(fn `OnWidgetHandStartInteraction`
  (params (HitResult :type "HitResult Structure (by ref)"))
  (bind _wic (`self.Wic`))
  (`ActorComponent.Activate` _wic false)
  (`WidgetInteractionComponent.SetCustomHitResult` _wic HitResult)
  (bind _returnvalue (`self.IfOverWidgetUse` true true))
  (if _returnvalue
    (`self.RumbleController` (`self.WidgetHapticEffect`))))

(fn `UserConstructionScript`)